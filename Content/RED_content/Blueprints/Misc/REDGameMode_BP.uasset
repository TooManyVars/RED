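; Game mode that runs menus, score, play timer and player respawns.
; BeginPlay opens the main menu and applies mostly low scalability settings.
; Once the game starts, Tick rebuilds the HUD every frame, shows the pause menu when paused, and updates high score and top time.
; RespawnPlayer destroys weapons, health pickups and enemies, spawns and possesses an armed player, and resets score and the CountUp-driven timer.
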(event Custom|RespawnPlayer
  (bind _outactors (Actor|GetAllActorsOfClass "/Game/RED_content/Blueprints/Player/Weapon.Weapon_C"))
  (for _array_element _outactors
    (Actor|DestroyActor _array_element))
  (bind _outactors_2 (Actor|GetAllActorsOfClass "/Game/RED_content/Blueprints/Misc/Pickups/FloatingHealthPickup.FloatingHealthPickup_C"))
  (for _array_element_2 _outactors_2
    (Actor|DestroyActor _array_element_2))
  (bind _outactors_3 (Actor|GetAllActorsOfClass "/Game/RED_content/Blueprints/Enemies/Enemy.Enemy_C"))
  (for _array_element_3 _outactors_3
    (Actor|DestroyActor _array_element_3))
  (bind _returnvalue (Game|SpawnActorfromClass "/Game/RED_content/Blueprints/Player/Player.Player_C" (Variables|Default|GetSpawnTransform) "Undefined" 0 0))
  (bind _aspc_bp (Utilities|Casting|CastToPC_BP (Game|GetPlayerController 0)))
  (Pawn|Possess _aspc_bp _returnvalue)
  (Input|EnableInput _returnvalue _aspc_bp)
  (bind _asplayer (Utilities|Casting|CastToPlayer (Game|GetPlayerCharacter 0)))
  (bind _output_get (Variables|Default|SetPlayer _asplayer))
  (Default|AttachGun _output_get)
  (Variables|Default|SetScore 0)
  (Variables|Default|Setseconds 0)
  (Variables|Default|Setminutes 0)
  (Variables|Default|Sethours 0)
  ;[1 1 1] Setting the variable to true allows the player to somehow pause the game after respawning
  (bind _asplayer_2 (Utilities|Casting|CastToPlayer (Game|GetPlayerCharacter 0)))
  (Variables|/Game/RED_content/Blueprints/Player/Player.Player_C|SetGameStarted _asplayer_2 true))

(event Custom|StartTimers
  (Utilities|Time|SetTimerbyFunctionName 0 "CountUp" 1.0 true))

(event Custom|Increment%20score
  (params (Delta :type Integer))
  (Variables|Default|SetScore (+ (Variables|Default|GetScore) Delta)))

(event EventBeginPlay
  (bind _returnvalue (UserInterface|CreateWidget "/Game/RED_content/Blueprints/UI/MainMenu.MainMenu_C"))
  (UserInterface|Viewport|AddtoViewport _returnvalue 0)
  (Development|ExecuteConsoleCommand "stat fps")
  (Development|ExecuteConsoleCommand "sg.ViewDistancQuality 0")
  (Development|ExecuteConsoleCommand "sg.ResolutionQuality 65")
  (Development|ExecuteConsoleCommand "sg.AntiAliasingQuality 0")
  (Development|ExecuteConsoleCommand "sg.EffectsQuality 1")
  (Development|ExecuteConsoleCommand "sg.PostProcessQuality 0")
  (Development|ExecuteConsoleCommand "sg.ShadowQuality 0")
  (Development|ExecuteConsoleCommand "sg.TextureQuality 0"))

(event EventTick
  (params (DeltaSeconds :type Float%20%28single-precision%29))
  (bind _asplayer (Utilities|Casting|CastToPlayer (Game|GetPlayerCharacter 0)))
  (if (Variables|/Game/RED_content/Blueprints/Player/Player.Player_C|GetGameStarted _asplayer)
    (Utilities|FlowControl|Sequence
      (:then_0
        (Viewport|RemoveAllWidgets)
        (bind _returnvalue (UserInterface|CreateWidget "/Game/RED_content/Blueprints/UI/HUD.HUD_C"))
        (UserInterface|Viewport|AddtoViewport _returnvalue 0))
      (:then_1
        ;[1 1 1] Constantly check whether or not the player has pressed p to pause the game(indicated by whether bIsPaused is true or not.
        (if (Variables|Default|GetbIsPaused)
          (Viewport|RemoveAllWidgets)
          (bind _returnvalue_2 (UserInterface|CreateWidget "/Game/RED_content/Blueprints/UI/PauseMenu.PauseMenu_C"))
          (UserInterface|Viewport|AddtoViewport _returnvalue_2 0)
          (Game|SetGamePaused true)
          (bind _aspc_bp (Utilities|Casting|CastToPC_BP (Game|GetPlayerController 0)))
          (bind _output_get (Variables|Default|SetPlayer%20controller _aspc_bp))
          (Variables|/Script/Engine.PlayerController|SetbShowMouseCursor _output_get true)))
      (:then_2
        ;[1 1 1] Keep checking to see whether the score has exceeded the high score. if so, make that the new high score.
        (if (> (Variables|Default|GetScore) (Variables|Default|GetHighScore))
          (Variables|Default|SetHighScore (Variables|Default|GetScore))))
      (:then_3
        (if (> (Variables|Default|Getseconds) (Variables|Default|GetTopSeconds))
          (if (>= (Variables|Default|Getseconds) (Variables|Default|GetTopSeconds))
            (if (>= (Variables|Default|Getminutes) (Variables|Default|GetTopMinutes))
              (if (>= (Variables|Default|Gethours) (Variables|Default|GetTopHours))
                (Variables|Default|SetTopSeconds (Variables|Default|Getseconds))
                (Variables|Default|SetTopMinutes (Variables|Default|Getminutes))
                (Variables|Default|SetTopHours (Variables|Default|GetTopHours))
                (if (== (Variables|Default|GetTopSeconds) 59)
                  (Variables|Default|SetTopSeconds 0)
                  (if (== (Variables|Default|GetTopMinutes) 59)
                    (Variables|Default|SetTopMinutes 0)
                    (if (== (Variables|Default|GetTopHours) 59)
                      (Variables|Default|SetTopHours 0))))))))))))

(fn ConstructionScript)

(fn CountUp
  (bind _output_get (Variables|Default|Setseconds (+ (Variables|Default|Getseconds) 1)))
  (if (> _output_get 59)
    (Variables|Default|Setseconds 0)
    (bind _output_get_2 (Variables|Default|Setminutes (+ (Variables|Default|Getminutes) 1)))
    (if (> _output_get_2 59)
      (Variables|Default|Setminutes 0)
      (Variables|Default|Sethours (+ (Variables|Default|Gethours) 1)))))

(fn CountUpTop
  (bind _output_get (Variables|Default|SetTopSeconds (+ (Variables|Default|GetTopSeconds) 1)))
  (if (> _output_get 59)
    (Variables|Default|SetTopSeconds 0)
    (bind _output_get_2 (Variables|Default|SetTopMinutes (+ (Variables|Default|GetTopMinutes) 1)))
    (if (> _output_get_2 59)
      (Variables|Default|SetTopMinutes 0)
      (Variables|Default|SetTopHours (+ (Variables|Default|GetTopHours) 1)))))