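; Player Blueprint for the RED game that handles weapon attachment, firing, health and respawning.
; Input stays disabled until GameStarted, when Tick spawns a weapon once onto the mesh's GunSocket and enables input.
; Fire input starts looping timers for shots and laser sound, gated by a DoOnce reset on release.
; Death destroys player and weapon after requesting a game-mode respawn at the saved start transform; Pause sets a game-mode flag.
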(event Custom|Pull%20trigger
  (Utilities|FlowControl|DoOnce false
    (:Completed
      (Audio|PlaySoundatLocation "/Game/RED_content/Blueprints/Misc/LaserSound.LaserSound" "0, 0, 0")
      (Class|PlayerCharacter|Fire)
      (Utilities|Time|SetTimerbyFunctionName 0 "Fire" (/ 1.0 (Variables|Default|GetRounds%20per%20second)) true)
      (Utilities|Time|SetTimerbyFunctionName 0 "GunFireNoise" (/ 1.0 (Variables|Default|GetRounds%20per%20second)) true))))

(event Custom|AttachGun
  (bind _mesh (Variables|Character|GetMesh))
  (bind _returnvalue (Game|SpawnActorfromClass "/Game/RED_content/Blueprints/Player/Weapon.Weapon_C" (Transformation|GetWorldTransform _mesh) "Undefined" 0 0))
  (bind _output_get (Variables|Default|SetWeapon _returnvalue))
  (Transformation|AttachComponentToComponent _output_get _mesh "GunSocket" "SnapToTarget" "SnapToTarget" "KeepRelative" true))

(event Custom|Release%20trigger
  (Utilities|Time|ClearTimerbyFunctionName 0 "GunFireNoise")
  (Utilities|Time|ClearTimerbyFunctionName 0 "Fire")
  (Utilities|FlowControl|DoOnce false) ; enters at Reset
)

(event EventBeginPlay
  (Variables|Default|SetMuzzleOffset "120.000000,35.000000,-45.000000")
  (Variables|Default|SetHealth 5e+02)
  (Input|DisableInput 0)
  (Utilities|FlowControl|Sequence
    (:then_1
      ;[1 1 1] Set the respawn transform variable within the game mode.
      (bind _asredgame_mode_bp (Utilities|Casting|CastToREDGameMode_BP (Game|GetGameMode)))
      (bind _output_get (Variables|Default|SetGameMode _asredgame_mode_bp))
      (Variables|/Game/RED_content/Blueprints/Misc/REDGameMode_BP.REDGameMode_BP_C|SetSpawnTransform _output_get (Transformation|GetActorTransform)))))

(event Collision|EventActorBeginOverlap
  (params (OtherActor :type Actor%20Object%20Reference)))

(event EventAffectHealth
  (params (Delta :type Float%20%28single-precision%29))
  ;[1 1 1] implmentation of the player's ability to take damage
  (Class|OurHero|RemainingHealth Delta)
  (Development|PrintString (Utilities|String|ToString(Float) (Variables|Default|GetHealth)) false)
  (Class|OurHero|CheckDead)
  (if (Variables|Default|GetIsDead)
    (Default|RespawnPlayer (Variables|Default|GetGameMode))
    (Actor|DestroyActor)
    (Actor|DestroyActor (Variables|Default|GetWeapon))))

(event EventTick
  (params (DeltaSeconds :type Float%20%28single-precision%29))
  ;[1 1 1] Attachment of the gun to the player character.
  (if (Variables|Default|GetGameStarted)
    (Utilities|FlowControl|DoOnce false
      (:Completed
        (CallFunction|AttachGun)
        (Input|EnableInput 0)))))

(event Input|ActionEvents|InputActionFire
  (params (Key :type Key%20Structure))
  (:Pressed
    (CallFunction|PullTrigger))
  (:Released
    (CallFunction|ReleaseTrigger)))

(event Input|ActionEvents|InputActionPause
  (params (Key :type Key%20Structure))
  ;[1 1 1] Set up part of the pause functionality within the player BP.
  (:Pressed
    (Variables|/Game/RED_content/Blueprints/Misc/REDGameMode_BP.REDGameMode_BP_C|SetbIsPaused (Variables|Default|GetGameMode) true)
    (Development|PrintText "Attempt was made to pause." false)))

(fn ConstructionScript)

(fn GunFireNoise
  (Audio|PlaySound2D "/Game/RED_content/Blueprints/Misc/LaserSound.LaserSound" 0.45))