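; Player bullet actor that damages what it hits in the game.
; On overlap, it checks that the other actor implements the IDamageable interface and lacks the Player and Pickup tags.
; It then sends its Damage value through AffectHealthMessage, spawns the EnemySparks emitter at its own position and destroys itself.
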(event EventBeginPlay)

(event EventTick
  (params (DeltaSeconds :type Float%20%28single-precision%29)))

(event Collision|EventActorBeginOverlap
  (params (OtherActor :type Actor%20Object%20Reference))
  (bind _returnvalue (Transformation|GetActorTransform))
  (if (Utilities|DoesObjectImplementInterface OtherActor "/Game/RED_content/Blueprints/Misc/IDamageable.IDamageable_C")
    (if (not (Actor|ActorHasTag OtherActor "Player"))
      (if (not (Actor|ActorHasTag OtherActor "Pickup"))
        (Class|IDamageable|AffectHealth(Message) OtherActor (Variables|Default|GetDamage))
        (Effects|SpawnEmitteratLocation "/Game/RED_content/FX/EnemySparks.EnemySparks" (.location _returnvalue) (.rotation _returnvalue))
        (Actor|DestroyActor)))))

(fn ConstructionScript)