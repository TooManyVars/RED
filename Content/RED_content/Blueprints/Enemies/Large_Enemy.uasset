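; Large enemy Blueprint, a child class that sets its own health, negative damage value and score award on BeginPlay.
; After setting these stats it calls ScaleDiffNoLog once.
; Tick runs the parent logic, then feeds a 60-second Delay into ScaleDifficulty, so difficulty scaling repeats roughly once a minute while the enemy exists.
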(event EventBeginPlay
  (|CallParentFunction)
  (Variables|Default|SetHealth 351.0)
  (Variables|Default|SetEnemyDamage -1.5e+02)
  (Variables|Default|SetScoreAwarded 250)
  (CallFunction|ScaleDiffNoLog))

(event Collision|EventActorBeginOverlap
  (params (OtherActor :type Actor%20Object%20Reference)))

(event EventTick
  (params (DeltaSeconds :type Float%20%28single-precision%29))
  (|CallParentFunction DeltaSeconds)
  (Utilities|FlowControl|Delay 6e+01)
  (CallFunction|ScaleDifficulty))

(fn ConstructionScript
  (|CallParentFunction))