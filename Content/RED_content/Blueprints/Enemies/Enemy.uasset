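; Enemy character Blueprint that damages the player in proximity, takes damage through AffectHealth, and on death awards score once before destroying itself after a delay.
; A DamageBox overlap runs a looping HitPlayer timer at the DPS rate.
; BeginPlay scales health, damage and walk speed by game-mode minutes and DifficultyMultiplier; a Delay on Tick repeats this each minute, but stores only speed, merely logging the others.
; Construction tints a dynamic material with EnemyColor.
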(event OnComponentBeginOverlap(DamageBox)
  (params (OverlappedComponent :type Primitive%20Component%20Object%20Reference) (OtherActor :type Actor%20Object%20Reference) (OtherComp :type Primitive%20Component%20Object%20Reference) (OtherBodyIndex :type Integer) (bFromSweep :type Boolean) (SweepResult :type Hit%20Result%20Structure%20%28by%20ref%29))
  ;[1 1 1] Functionality that allows the enemy to hit the player once they enter proximiy.
  (bind _asplayer (Utilities|Casting|CastToPlayer OtherActor))
  (Variables|Default|SetPlayer%20character _asplayer)
  (Utilities|Time|SetTimerbyFunctionName 0 "HitPlayer" (/ 1.0 (Variables|Default|GetDPS)) true))

(event OnComponentEndOverlap(DamageBox)
  (params (OverlappedComponent :type Primitive%20Component%20Object%20Reference) (OtherActor :type Actor%20Object%20Reference) (OtherComp :type Primitive%20Component%20Object%20Reference) (OtherBodyIndex :type Integer))
  ;[1 1 1] Functionality that allows the enemy to hit the player once they enter proximiy.
  (if (== OtherActor (Variables|Default|GetPlayer%20character))
    (Utilities|Time|ClearTimerbyFunctionName 0 "HitPlayer")))

(event Custom|HitPlayer
  ;[1 1 1] Functionality that allows the enemy to hit the player once they enter proximiy.
  (Default|AffectHealth (Variables|Default|GetPlayer%20character) (Variables|Default|GetEnemyDamage)))

(event EventBeginPlay
  ;[1 1 1] Recalculate the health at the beginning of the enemy's life(ctrl-c'ed the code because i couldn't put parameters into the function timer).
  (Variables|Default|SetHealth 1e+02)
  ;;[1 1 1] i made a completely  different logging function because i don't want a log being made everytime an enemy spawns
  (CallFunction|ScaleDiffNoLog))

(event EventTick
  (params (DeltaSeconds :type Float%20%28single-precision%29))
  ;[1 1 1] Every minute or so, the health, damage and speed of the enemies are recalculated. requires some testing.
  (Utilities|FlowControl|Delay 6e+01)
  (CallFunction|ScaleDifficulty))

(event EventAffectHealth
  (params (Delta :type Float%20%28single-precision%29))
  (bind _capsulecomponent (Variables|Default|GetCapsuleComponent))
  ;[1 1 1] Implementation of IDamagable in which the enemy will take damage and will have the rest of it's health printed to the screen with loiw enough health it will die,
  (Class|OurHero|RemainingHealth Delta)
  (Development|PrintString (Utilities|String|ToString(Float) (Variables|Default|GetHealth)) false)
  (Class|OurHero|CheckDead)
  (if (Variables|Default|GetIsDead)
    (Utilities|FlowControl|Sequence
      (:then_0
        (Utilities|FlowControl|DoOnce false
          (:Completed
            (bind _asredgame_mode_bp (Utilities|Casting|CastToREDGameMode_BP (Game|GetGameMode)))
            (Default|IncrementScore _asredgame_mode_bp (Variables|Default|GetScoreAwarded)))))
      (:then_1
        (Collision|SetCollisionResponsetoChannel _capsulecomponent "ECC_WorldDynamic" "ECR_Ignore")
        (Collision|SetCollisionResponsetoChannel _capsulecomponent "ECC_Pawn" "ECR_Ignore")
        (Class|Pawn|DetachfromControllerPendingDestroy)
        (Utilities|FlowControl|Delay 3.0)
        (Actor|DestroyActor)))))

(fn ConstructionScript
  (bind _returnvalue (Rendering|Material|CreateDynamicMaterialInstance (Variables|Character|GetMesh) 0 0 :!class /Script/Engine.PrimitiveComponent))
  (bind _output_get (Variables|Default|SetDyna%20material _returnvalue))
  (Rendering|Material|SetVectorParameterValue _output_get "EnemyColor" (* (Variables|Default|GetEnemyColor) 5.0) :!class /Script/Engine.MaterialInstanceDynamic))

(fn IncreaseValues
  (params (InAttribute :type Integer))
  (bind _asredgame_mode_bp (Utilities|Casting|CastToREDGameMode_BP (Game|GetGameMode)))
  (return (+ (* (Variables|/Game/RED_content/Blueprints/Misc/REDGameMode_BP.REDGameMode_BP_C|Getminutes _asredgame_mode_bp) (Variables|Default|GetDifficultyMultiplier)) InAttribute)))

(fn LogNewValue
  (params (Value :type Integer))
  (Development|PrintString (Utilities|String|ToString(Text) (Utilities|Text|FormatText "New value is: {v}" Value)) false))

(fn IncreaseEnemyDamage
  (params (CurrentDamage :type Integer))
  (bind _asredgame_mode_bp (Utilities|Casting|CastToREDGameMode_BP (Game|GetGameMode)))
  (return (- CurrentDamage (* (Variables|/Game/RED_content/Blueprints/Misc/REDGameMode_BP.REDGameMode_BP_C|Getminutes _asredgame_mode_bp) (Variables|Default|GetDifficultyMultiplier)))))

(fn ScaleDifficulty
  (bind _newdamage (CallFunction|IncreaseEnemyDamage (Math|Float|Truncate (Variables|Default|GetEnemyDamage))))
  (CallFunction|LogNewValue (Math|Float|Truncate (Math|Conversions|ToFloat(Integer) _newdamage)))
  (bind _outattribute (CallFunction|IncreaseValues (Math|Float|Truncate (Variables|/Script/Engine.CharacterMovementComponent|GetMaxWalkSpeed (Variables|Character|GetCharacterMovement)))))
  (bind _output_get (Variables|/Script/Engine.CharacterMovementComponent|SetMaxWalkSpeed (Variables|Character|GetCharacterMovement) (Math|Conversions|ToFloat(Integer) _outattribute)))
  (CallFunction|LogNewValue (Math|Float|Truncate _output_get))
  (bind _outattribute_2 (CallFunction|IncreaseValues (Math|Float|Truncate (Variables|Default|GetHealth))))
  (CallFunction|LogNewValue (Math|Float|Truncate (Math|Conversions|ToFloat(Integer) _outattribute_2))))

(fn ScaleDiffNoLog
  (bind _newdamage (CallFunction|IncreaseEnemyDamage (Math|Float|Truncate (Variables|Default|GetEnemyDamage))))
  (Variables|Default|SetEnemyDamage (Math|Conversions|ToFloat(Integer) _newdamage))
  (bind _outattribute (CallFunction|IncreaseValues (Math|Float|Truncate (Variables|/Script/Engine.CharacterMovementComponent|GetMaxWalkSpeed (Variables|Character|GetCharacterMovement)))))
  (Variables|/Script/Engine.CharacterMovementComponent|SetMaxWalkSpeed (Variables|Character|GetCharacterMovement) (Math|Conversions|ToFloat(Integer) _outattribute))
  (bind _outattribute_2 (CallFunction|IncreaseValues (Math|Float|Truncate (Variables|Default|GetHealth))))
  (Variables|Default|SetHealth (Math|Conversions|ToFloat(Integer) _outattribute_2)))