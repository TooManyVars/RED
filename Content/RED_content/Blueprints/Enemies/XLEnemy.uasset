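; XLEnemy is an enemy Blueprint with high health and a score award, whose damage grows with the number of enemies in the level.
; BeginPlay sets its stats and calls ScaleDiffNoLog.
; Tick recomputes EnemyDamage from DamageMultiplier and the count of Enemy-tagged actors, so killing others weakens it.
; A Delay within Tick gates ScaleDifficulty to run about once a minute.
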(event EventBeginPlay
  (|CallParentFunction)
  (Variables|Default|SetHealth 1.25e+03)
  (Variables|Default|SetScoreAwarded 500)
  (CallFunction|ScaleDiffNoLog))

(event Collision|EventActorBeginOverlap
  (params (OtherActor :type Actor%20Object%20Reference)))

(event EventTick
  (params (DeltaSeconds :type Float%20%28single-precision%29))
  ;[1 1 1] The whole point of this enemy is that the more enemies in the level there are, the more damage they do. kill other enemies in the level in order to reduce the amount of damge it does.
  (|CallParentFunction DeltaSeconds)
  (bind _outactors (Actor|GetAllActorswithTag "Enemy"))
  (Variables|Default|SetEnemyDamage (Math|Conversions|ToFloat(Integer) (* (Variables|Default|GetDamage%20multiplier) (Utilities|Array|Length _outactors))))
  (Utilities|FlowControl|Delay 6e+01)
  (CallFunction|ScaleDifficulty))

(fn ConstructionScript
  (|CallParentFunction))