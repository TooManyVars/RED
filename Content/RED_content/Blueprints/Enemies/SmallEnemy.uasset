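; SmallEnemy is a child enemy Blueprint that sets its own damage, health and score on BeginPlay, then calls ScaleDiffNoLog.
; Each Tick counts all SmallEnemy actors and, while SmallEnemyRequirement is at least that count, adds DamageBoost to the truncated Damage.
; That branch then calls ScaleDifficulty after a one-minute Delay.
; The comparison runs opposite to the author's note, which intends the boost for large groups.
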(event EventBeginPlay
  (|CallParentFunction)
  (Variables|Default|SetEnemyDamage -25.0)
  (Variables|Default|SetHealth 25.0)
  (Variables|Default|SetScoreAwarded 100)
  (CallFunction|ScaleDiffNoLog))

(event Collision|EventActorBeginOverlap
  (params (OtherActor :type Actor%20Object%20Reference)))

(event EventTick
  (params (DeltaSeconds :type Float%20%28single-precision%29))
  ;[1 1 1] The whole purpose of the smaller enemy is that if there are more than 10 in the level,  each enemy gets a damage boost of 30.
  (|CallParentFunction DeltaSeconds)
  (bind _outactors (Actor|GetAllActorsOfClass "SmallEnemy_C"))
  (if (>= (Variables|Default|GetSmall%20enemy%20requirement) (Utilities|Array|Length _outactors))
    (Variables|Default|SetDamage (Math|Conversions|ToFloat(Integer) (+ (Variables|Default|GetDamage%20boost) (Math|Float|Truncate (Variables|Default|GetDamage)))))
    (Utilities|FlowControl|Delay 6e+01)
    (CallFunction|ScaleDifficulty)))

(fn ConstructionScript
  (|CallParentFunction))